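; BP_PurpleDragon is a dragon character that heads for a treasure point with a periodic backward-step behavior.
; MovetoTreasurePoint starts an AI move toward TreasureRef and a looping timer that fires WalkBackTime during the trip.
; Each tick of that timer halts movement while keeping the path, plays a walk-back montage, then restores walking after a short delay.
; Reaching the treasure pauses the timer and calls GetTreasure.
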(event Custom|WalkBackTime
  (bind _charactermovement (Variables|Character|GetCharacterMovement))
  ;[1 1 1] setting timer for step backward every second
  (Class|NavMovementComponent|StopMovementKeepPathing _charactermovement)
  (Pawn|Components|CharacterMovement|DisableMovement _charactermovement)
  (Animation|PlayAnimMontage "/Game/Characters/Purple/AM_Purple_WalkBack.AM_Purple_WalkBack" 1.0 "None")
  (Utilities|FlowControl|Delay 0.5)
  (Pawn|Components|CharacterMovement|SetMovementMode (Variables|Character|GetCharacterMovement) "MOVE_Walking" 0))

(event EventBeginPlay
  (|CallParentFunction) ; This node is disabled and will not be called.\nDrag off pins to build functionality.
)

(event Collision|EventActorBeginOverlap
  (params (OtherActor :type Actor%20Object%20Reference)))

(event EventTick
  (params (DeltaSeconds :type Float%20%28single-precision%29)))

(event EventMovetoTreasurePoint
  (AI|AIMoveTo self "0, 0, 0" (Variables|Default|GetTreasureRef) 5.0 false
    (:then
      ;[1 1 1] setting timer for step backward every second
      (bind _returnvalue (Utilities|Time|SetTimerbyEvent (delegate Custom|WalkBackTime) 1.5 true -1.0))
      (Variables|Default|SetWalkBackwardTimer _returnvalue))
    (:OnSuccess
      (Utilities|Time|PauseTimerbyHandle (Variables|Default|GetWalkBackwardTimer))
      (CallFunction|GetTreasure 3.0))))

(fn ConstructionScript
  (|CallParentFunction))