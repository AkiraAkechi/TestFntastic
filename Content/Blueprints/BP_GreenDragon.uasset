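; BP_GreenDragon is a dragon character that walks to a treasure target, stopping periodically along the way.
; MovetoTreasurePoint starts an AI MoveTo toward TreasureRef and a looping timer that fires WaitTime.
; Each WaitTime disables movement while keeping the path, plays a wait montage, then restores walking after a short delay.
; On arrival, it pauses the timer and calls GetTreasure.
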(event Custom|WaitTime
  (bind _charactermovement (Variables|Character|GetCharacterMovement))
  ;[1 1 1] Set timer for waitin every second
  (Class|NavMovementComponent|StopMovementKeepPathing _charactermovement)
  (Pawn|Components|CharacterMovement|DisableMovement _charactermovement)
  (Animation|PlayAnimMontage "/Game/Characters/Green/AM_Green_Wait.AM_Green_Wait" 1.0 "None")
  (Utilities|FlowControl|Delay 0.5)
  (Pawn|Components|CharacterMovement|SetMovementMode (Variables|Character|GetCharacterMovement) "MOVE_Walking" 0))

(event EventBeginPlay
  (|CallParentFunction) ; This node is disabled and will not be called.\nDrag off pins to build functionality.
)

(event EventMovetoTreasurePoint
  (AI|AIMoveTo self "0, 0, 0" (Variables|Default|GetTreasureRef) 1e+02 false
    (:then
      ;[1 1 1] Set timer for waitin every second
      (bind _returnvalue (Utilities|Time|SetTimerbyEvent (delegate Custom|WaitTime) 1.5 true -1.0))
      (Variables|Default|SetWaitingTimer _returnvalue))
    (:OnSuccess
      (Utilities|Time|PauseTimerbyHandle (Variables|Default|GetWaitingTimer))
      (CallFunction|GetTreasure 3.0))))

(fn ConstructionScript
  (|CallParentFunction))