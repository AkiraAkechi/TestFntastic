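; Base dragon character that travels to the treasure matching its dragon type and claims it.
; On BeginPlay it finds its treasure by a type-based actor tag, then calls MoveToTreasurePoint once the spawn montage completes.
; GetTreasure glides the capsule to the treasure's seating point during a montage.
; When that montage completes, it notifies its button that movement ended, plays smoke and sound effects, then destroys itself.
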(event Custom|GetTreasure
  (params (MoveOverTime :type Float%20%28single-precision%29))
  (bind _treasureref (Variables|Refs|GetTreasureRef))
  (bind _dragonseetingpoint (Variables|/Game/Blueprints/BP_Treasure.BP_Treasure_C|GetDragonSeetingPoint _treasureref))
  (bind _returnvalue (Transformation|GetWorldTransform _dragonseetingpoint))
  ;[1 1 1] Find treasure event
  (Animation|Montage|PlayMontage (Variables|Character|GetMesh) (Variables|Montages|GetFindTreasureAnumMontage)
    (:then
      (Components|MoveComponentTo (Variables|Collision|GetCapsuleComponent) (.location _returnvalue) (.rotation _returnvalue) true true MoveOverTime false) ; Move character on the treasure while montage playing
    )
    (:OnCompleted
      (Class|BPIInteraction|OnDragonEndMove(Message) (Variables|Refs|GetButtonRef) (Variables|Default|GetDragonType)) ; call button, what dragon end moving for unlock
      (Niagara|SpawnSystematLocation "/Game/sA_Megapack_v1/NS_Smoke_Explosion.NS_Smoke_Explosion" (.location _returnvalue) (.rotation _returnvalue))
      (Audio|PlaySound2D "/Game/Characters/Sound/mixkit-bonus-earned-in-video-game-2058.mixkit-bonus-earned-in-video-game-2058" 0.5 1.0 0.0 0 0)
      (Utilities|FlowControl|Delay 0.1)
      (Actor|DestroyActor))))

(event EventBeginPlay
  ;[1 1 1] Set Treasure Ref
  (bind _outactors (Actor|GetAllActorswithTag (Utilities|Select :Index (Variables|Default|GetDragonType) :NewEnumerator0 "RedDragon" :NewEnumerator1 "GreenDragon" :NewEnumerator2 "PurpleDragon")))
  (bind _asbp_treasure (Utilities|Casting|CastToBP_Treasure (Utilities|Array|Get(acopy) _outactors)))
  (Variables|Refs|SetTreasureRef _asbp_treasure)
  ;[1 1 1] Play Anim montage on Spawned
  (Animation|Montage|PlayMontage (Variables|Character|GetMesh) (Variables|Montages|GetSpawnedAnimMontage)
    (:OnCompleted
      ;[1 1 1] call to start moving
      (CallFunction|MovetoTreasurePoint))))

(fn ConstructionScript)