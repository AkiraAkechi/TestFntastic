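; BP_InteractiveButton is a clickable button tied to one dragon type, with its gem material (ruby, emerald or amethyst) set from that type on BeginPlay.
; A click plays a sound, lowers the activator and messages every BPI_Interaction actor with the type and a self reference to trigger dragon spawners.
; A DoOnce locks the button until OnDragonEndMove receives the matching type, which raises it, plays a sound and re-arms it.
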(event OnClicked(ButtonActivator)
  (params (TouchedComponent :type Primitive%20Component%20Object%20Reference) (ButtonPressed :type Key%20Structure :default "None"))
  (Utilities|FlowControl|DoOnce false
    (:Completed
      (Audio|PlaySound2D "/Engine/VREditor/Sounds/UI/Click_on_Button.Click_on_Button" 1.0 1.0 0.0 0 0)
      (Components|MoveComponentTo (Variables|Default|GetButtonActivator) "0, 0, 0" "0, 0, 0" true true 0.5 false)
      ;[1 1 1] Call  dragon spawners
      (bind _outactors (Actor|GetAllActorswithInterface "/Game/Blueprints/BPI_Interaction.BPI_Interaction_C"))
      (for _array_element _outactors
        (Class|BPIInteraction|OnClickButton(Message) _array_element (Variables|Default|GetSpawningDragonType) self)))))

(event EventBeginPlay
  ;[1 1 1] change button color by dragon type
  (Rendering|Material|SetMaterial (Variables|Default|GetButtonActivator) 0 (Utilities|Select :Index (Variables|Default|GetSpawningDragonType) :NewEnumerator0 "/Game/LPSDeluxe2TropicalEnvironment/LPSD2_Materials/Materials/Master_Color_Instances/MI_Gem_Ruby.MI_Gem_Ruby" :NewEnumerator1 "/Game/LPSDeluxe2TropicalEnvironment/LPSD2_Materials/Materials/Master_Color_Instances/MI_Gem_Emerald.MI_Gem_Emerald" :NewEnumerator2 "/Game/LPSDeluxe2TropicalEnvironment/LPSD2_Materials/Materials/Master_Color_Instances/MI_Gem_Amethyst.MI_Gem_Amethyst")))

(event EventOnDragonEndMove
  (params (DragonType :type ENUM_DragonType%20Enum :default "NewEnumerator0"))
  ;[1 1 1] unlock button, when dragon end moving
  (if (Utilities|Enum|Equal(Enum) DragonType (Variables|Default|GetSpawningDragonType))
    (Components|MoveComponentTo (Variables|Default|GetButtonActivator) "0, 0,80.000000" "0, 0, 0" true true 0.5 false)
    (Audio|PlaySound2D "/Game/Characters/Sound/mixkit-game-ball-tap-2073.mixkit-game-ball-tap-2073" 1.0 1.0 0.0 0 0)
    (Utilities|FlowControl|DoOnce false) ; enters at Reset
  ))

(fn ConstructionScript)