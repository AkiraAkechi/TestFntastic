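; BP_DragonSpawner is a spawner actor that creates a red, green or purple dragon according to its DragonType.
; BeginPlay swaps its static mesh to one matching that type.
; OnClickButton responds only to a matching dragon type, spawning that pawn at SpawnPoint with the button reference passed in.
; It then gives the pawn its default controller and plays a scaled-up Niagara spawn effect at the same spot.
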(event EventBeginPlay
  ;[1 1 1] change spawner vesh by dragon type
  (Components|StaticMesh|SetStaticMesh (Variables|Default|GetStaticMesh) (Utilities|Select :Index (Variables|Default|GetDragonType) :NewEnumerator0 "/Game/LPSDeluxe2TropicalEnvironment/LPSD2_Meshes/Pirate/SM_PirateChest_2.SM_PirateChest_2" :NewEnumerator1 "/Game/LPSDeluxe2TropicalEnvironment/LPSD2_Meshes/Water/SM_WaterFallSplash_2.SM_WaterFallSplash_2" :NewEnumerator2 "/Game/LPSDeluxe2TropicalEnvironment/LPSD2_Meshes/Pirate/SM_ShipBarrel_3.SM_ShipBarrel_3")))

(event EventOnClickButton
  (params (ButtonDragonType :type ENUM_DragonType%20Enum :default "NewEnumerator0") (ButtonRef :type BP%20Interactive%20Button%20Object%20Reference))
  (bind _spawnpoint (Variables|Default|GetSpawnPoint))
  (bind _dragontype (Variables|Default|GetDragonType))
  (bind _returnvalue (Transformation|GetWorldTransform _spawnpoint))
  ;[1 1 1] Implement Button Click event
  (if (Utilities|Enum|Equal(Enum) ButtonDragonType _dragontype)
    (bind _output_get (Variables|Refs|SetPawnClass (Utilities|Select :Index _dragontype :NewEnumerator0 "/Game/Blueprints/BP_redDragon.BP_RedDragon_C" :NewEnumerator1 "/Game/Blueprints/BP_GreenDragon.BP_GreenDragon_C" :NewEnumerator2 "/Game/Blueprints/BP_PurpleDragon.BP_PurpleDragon_C")))
    (bind _returnvalue_2 (Game|SpawnActorfromClass _output_get _returnvalue "AdjustIfPossibleButAlwaysSpawn" 0 ButtonRef 0))
    (Pawn|SpawnDefaultController _returnvalue_2)
    (Niagara|SpawnSystematLocation "/Game/sA_Megapack_v1/NS_Spawn.NS_Spawn" (.Location (Math|Transform|BreakTransform _returnvalue)) "0, 0, 0" "10.000000,10.000000,10.000000")))

(fn ConstructionScript)